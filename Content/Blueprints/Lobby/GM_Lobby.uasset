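; Lobby game mode that registers joining players, spawns them as a base character and server-travels to the selected arena.
; PostLogin pulls server name and player limit from the game instance, initializes each PC_Lobby, then respawns it at a random PlayerStart.
; EveryoneUpdate pushes player lists, counts and available characters to all controllers and sets CanStart from character picks.
; Map setting changes are relayed to every controller; kick-list and character-swap events are empty stubs.
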(event Custom|SwapCharacter
  (params (PlayerController :type Player%20Controller%20Object%20Reference) (CharcterClass :type Character%20Class%20Reference) (ChangedStatus :type Boolean)))

(event Custom|RespawnPlayer
  (params (PlayerController :type Player%20Controller%20Object%20Reference))
  (bind _returnvalue (Pawn|GetControlledPawn PlayerController))
  (bind _spawnpoints (Variables|ServerSettings|GetSpawnPoints))
  ;[1 1 1] Spawn the player as base character when ariving at the Lobby Menu / Tells everyone to update thier lobbies
  (Utilities|IsValid _returnvalue
    (:Is%20Valid
      (Actor|DestroyActor _returnvalue))
    (:Is%20Not%20Valid
      _))
  (bind _returnvalue_2 (Game|SpawnActorfromClass "/Game/Blueprints/Character/0_Base.0_Base_C" (Transformation|GetActorTransform (Utilities|Array|Get(acopy) _spawnpoints (Math|Random|RandomIntegerinRange 0 (- (Utilities|Array|Length _spawnpoints) 1)))) "Undefined" 0 0))
  (Pawn|Possess PlayerController _returnvalue_2)
  (CallFunction|EveryoneUpdate))

(event Custom|LaunchTheGame
  (bind _returnvalue (Game|GetPlayerController 0))
  ;[1 1 1] Launch the game based on map selection in Game Settings
  (switch int (Variables|ServerSettings|GetGM_MapId)
    (:0
      (Development|ExecuteConsoleCommand "servertravel /Game/Maps/Arena01" _returnvalue))
    (:1
      (Development|ExecuteConsoleCommand "servertravel /Game/Maps/Arena02" _returnvalue))))

(event Custom|AddToKickList)

(event Custom|CannontStartGame
  ;[1 1 1] Update all connected players lobby info when called
  (Utilities|Array|ForEachLoopwithBreak (Variables|ServerSettings|GetConnectedPlayers)) ; enters at Break
)

(event Custom|ServerUpdateGameSettings
  (params (MapImage :type Texture%202D%20Object%20Reference) (MapName :type Text) (MapTime :type Text) (MapId :type Integer))
  ;[1 1 1] Server has made changes tell each client to update thier lobby info
  (Variables|ServerSettings|SetGM_MapImage MapImage)
  (Variables|ServerSettings|SetGM_MapName MapName)
  (Variables|ServerSettings|SetGM_MapTime MapTime)
  (Variables|ServerSettings|SetGM_MapId MapId)
  (for _array_element (Variables|ServerSettings|GetAllPlayerControllers)
    (bind _aspc_lobby (Utilities|Casting|CastToPC_Lobby _array_element))
    (Default|UpdateLobbySettings _aspc_lobby (Variables|ServerSettings|GetGM_MapImage) (Variables|ServerSettings|GetGM_MapName) (Variables|ServerSettings|GetGM_MapTime))))

(event Custom|EveryoneUpdate
  (bind _allplayercontrollers (Variables|ServerSettings|GetAllPlayerControllers))
  ;[1 1 1] Update all connected players lobby info when called
  (bind _output_get (Variables|ServerSettings|SetCurrentPlayers (Utilities|Array|Length (Variables|ServerSettings|GetAllPlayerControllers))))
  (if (> _output_get 0)
    (Utilities|Array|Clear (Variables|ServerSettings|GetConnectedPlayers))
    (for _array_element _allplayercontrollers
      (bind _aspc_lobby (Utilities|Casting|CastToPC_Lobby _array_element))
      (Utilities|Array|Add (Variables|ServerSettings|GetConnectedPlayers) (Variables|/Game/Blueprints/Lobby/PC_Lobby.PC_Lobby_C|GetPlayerSettings _aspc_lobby))
      (Default|UpdateNumberOfPlayers _aspc_lobby (Variables|ServerSettings|GetCurrentPlayers) (Variables|ServerSettings|GetMaxPlayers)))
    (for _array_element_2 _allplayercontrollers
      (bind _aspc_lobby_2 (Utilities|Casting|CastToPC_Lobby _array_element_2))
      (Default|AddPlayerInfo _aspc_lobby_2 (Variables|ServerSettings|GetConnectedPlayers))
      (Default|UpdateAvaliableCharacters _aspc_lobby_2 (Variables|ServerSettings|GetAvaliableCharacters))
      (CallFunction|AddtoKickList))
    (bind _array_element_3 (Utilities|Array|ForEachLoopwithBreak (Variables|ServerSettings|GetConnectedPlayers))
      (:LoopBody
        (if (== (.MyPlayerCharacter (Utilities|Struct|BreakPlayerInfo _array_element_3)) "/Game/Blueprints/Character/0_Base.0_Base_C")
          (Variables|ServerSettings|SetCanStart false)
          (CallFunction|CannontStartGame)
          (else
            (Variables|ServerSettings|SetCanStart true)))))))

(event EventPostLogin
  (params (NewPlayer :type Player%20Controller%20Object%20Reference))
  ;[1 1 1] Initial Setup occures on event post login - Handles lobby setup and spawns the player
  (Networking|SwitchHasAuthority
    (:Authority
      (Utilities|Array|Add (Variables|ServerSettings|GetAllPlayerControllers) NewPlayer)
      (bind _outactors (Actor|GetAllActorsOfClass "/Script/Engine.PlayerStart"))
      (Variables|ServerSettings|SetSpawnPoints _outactors)
      (bind _asgame_info_instance (Utilities|Casting|CastToGameInfoInstance (Game|GetGameInstance)))
      (Variables|ServerSettings|SetServerName (Variables|/Game/Blueprints/AllLevels/GameInfoInstance.GameInfoInstance_C|GetServerName _asgame_info_instance))
      (Variables|ServerSettings|SetMaxPlayers (Variables|/Game/Blueprints/AllLevels/GameInfoInstance.GameInfoInstance_C|GetMaxPlayers _asgame_info_instance))
      (bind _aspc_lobby (Utilities|Casting|CastToPC_Lobby NewPlayer))
      (Default|InitSetup _aspc_lobby)
      (Default|SetupLobbyMenu _aspc_lobby (Variables|ServerSettings|GetServerName))
      (Default|UpdateLobbySettings _aspc_lobby (Variables|ServerSettings|GetGM_MapImage) (Variables|ServerSettings|GetGM_MapName) (Variables|ServerSettings|GetGM_MapTime))
      (CallFunction|RespawnPlayer NewPlayer))))

(fn ConstructionScript)